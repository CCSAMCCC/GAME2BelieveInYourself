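; BP_WindowBlockLv2 is a window block that absorbs hits, apparently from hammers, and breaks after three.
; Each overlap on its Box component destroys the other actor without any type check, prints the current AmountOfHammers count as debug output, then increments it.
; Once the count reaches the threshold, the block destroys itself.
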(event `self.Box.OnComponentBeginOverlap`
  (params (OverlappedComponent :type "PrimitiveComponent Object Reference") (OtherActor :type "Actor Object Reference") (OtherComp :type "PrimitiveComponent Object Reference") (OtherBodyIndex :type Integer) (bFromSweep :type Boolean) (SweepResult :type "HitResult Structure (by ref)"))
  (`self.K2_DestroyActor` OtherActor)
  (`KismetSystemLibrary.PrintString` (`KismetStringLibrary.Conv_IntToString` (`self.amountOfHammers`)))
  (bind _result (`/Engine/EditorBlueprintResources/StandardMacros.IncrementInt` (`self.amountOfHammers`))
    (:`  `
      (set `self.amountOfHammers` _result)
      (if (>= (`self.amountOfHammers`) 3)
        (`self.K2_DestroyActor`)))))

(fn `UserConstructionScript`)