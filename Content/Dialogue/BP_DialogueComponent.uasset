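; Dialogue component that shows single typewriter lines or runs branching dialogue through Behavior Trees on the owner's AI controller.
; Single lines push a new WBP_DialogueBox onto the first-person player's ActiveDialogueDisplay stack.
; Dialogue trees run BTAsset and reveal that display on success, while stopping switches the AI back to the owner's default tree.
; It also holds a replaceable choice memory.
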(fn `RunDialogueTree`
  (returns (ReturnValue :type Boolean))
  (bind _returnvalue (`AIBlueprintHelperLibrary.GetAIController` (`self.GetOwner`)))
  (`/Engine/EditorBlueprintResources/StandardMacros.IsValid` _returnvalue
    (:`Is Valid`
      (bind _returnvalue_2 (`AIController.RunBehaviorTree` _returnvalue (`self.BTAsset`)))
      (if _returnvalue_2
        (bind _asbp_first_person_character (cast `/Game/FirstPerson/Blueprints/BP_FirstPersonCharacter` (`GameplayStatics.GetPlayerCharacter` 0)))
        (`Widget.SetVisibility` (`/Game/FirstPerson/Blueprints/BP_FirstPersonCharacter.Active Dialogue Display` _asbp_first_person_character) "Visible"))
      (return _returnvalue_2))
    (:`Is Not Valid`
      (return false))))

(fn `RunSingleDialogue`
  (params (Text :type Text) (`Typewriter Delay Between Letters` :type "Float (double-precision)" :default 0.1))
  (bind _asbp_first_person_character (cast `/Game/FirstPerson/Blueprints/BP_FirstPersonCharacter` (`GameplayStatics.GetPlayerCharacter` 0)))
  (bind _active_dialogue_display (`/Game/FirstPerson/Blueprints/BP_FirstPersonCharacter.Active Dialogue Display` _asbp_first_person_character))
  (`Widget.SetVisibility` _active_dialogue_display "Visible")
  (bind _returnvalue (`|CreateWidget` "/Game/Widgets/WBP_DialogueBox.WBP_DialogueBox_C" null Text `Typewriter Delay Between Letters`))
  (`/Game/Widgets/WBP_DialogueDisplay.AddWidgetToStack` _active_dialogue_display _returnvalue)
  (add `/Game/Widgets/WBP_DialogueDisplay.Textfinished` _active_dialogue_display (`|CreateDelegate` _asbp_first_person_character :!event `End DialogueDisplay`)))

(fn `Set Choice memeory `
  (params (`new memoery` :type "Map of Integer to Integer"))
  (`BlueprintMapLibrary.Map_Clear` (`self.ChoiceMemoery`))
  (set `self.ChoiceMemoery` `new memoery`))

(fn `Stop DialogueTree`
  (bind _returnvalue (`self.GetOwner`))
  (bind _bt_asset (message `/Game/Dialogue/BPI_Dialogue.Get Default BT Asset` _returnvalue))
  (`AIController.RunBehaviorTree` (`AIBlueprintHelperLibrary.GetAIController` _returnvalue) _bt_asset))