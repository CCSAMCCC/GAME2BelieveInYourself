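; BP_Scientist is a scientist actor that can hold a dialogue through its BPDialogueComponent.
; It supplies DT_Cornetta as its default BT asset, exposes the component through a getter, and forwards RunDialogue to the component's RunDialogueTree, returning the result.
; On BeginPlay it hides its Sphere component without affecting children; it has no other active event logic.
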(event `self.ReceiveBeginPlay`
  (`SceneComponent.SetVisibility` (`self.Sphere`) false false))

(fn `Get Default BT Asset`
  (returns (`BT Asset` :type "BehaviorTree Object Reference"))
  (return "/Game/Dialogue/DT_Cornetta.DT_Cornetta"))

(fn `GetDialogueComponent`
  (returns (DiagloeuComponent :type "/Game/Dialogue/BP_DialogueComponent Object Reference"))
  (return (`self.BP_DialogueComponent`)))

(fn `RunDialogue`
  (returns (Success :type Boolean))
  (bind _returnvalue (`/Game/Dialogue/BP_DialogueComponent.RunDialogueTree` (`self.BP_DialogueComponent`)))
  (return _returnvalue))

(fn `UserConstructionScript`)